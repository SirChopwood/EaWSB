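; Game instance Blueprint that hosts and joins multiplayer sessions using Advanced Sessions nodes.
; CreateSession creates a session and, on success, opens the SpaceSkirmish level as a listen server.
; FindSession searches all server types, stores the results and loops over them with an empty body, then calls JoinSession on the loop's last element.
; Search status is shown only through printed messages, and the join result is not handled.
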(event Custom|Find%20Session
  (bind _returnvalue (Game|GetPlayerController 0))
  (bind _results (|FindSessionsAdvanced _returnvalue 100 false "AllServers" 0 false false false)
    (:OnSuccess
      (Development|PrintString "Connecting to Server")
      (bind _output_get (Variables|Default|SetFoundSessions _results))
      (for _array_element _output_get
        _)
      (|JoinSession _returnvalue _array_element))
    (:OnFailure
      (Development|PrintString "No Servers Found"))))

(event Custom|Create%20Session
  (|AdvancedSession 0 (Game|GetPlayerController 0) 100 0 false true false true true false false false true
    (:OnSuccess
      (Game|OpenLevel(byName) "SpaceSkirmish" true "listen"))))